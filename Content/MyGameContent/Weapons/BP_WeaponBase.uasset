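; Base weapon class for the player, declaring stub events for fire, reload, throw, recoil, pose and HUD ammo.
; It caches BP_Player on BeginPlay and lowers the player's walk speed during aim or throw, restoring it afterward.
; Equip clears aim and fire state, then chains unequip and equip montages around a socket swap between hand and back.
; Finally, it sets the new current weapon and refreshes its pose and ammo HUD.
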(event Custom|Fire
  (params (Fire :type Boolean)))

(event Custom|Reload)

(event Custom|WeaponRecoil)

(event Custom|Equip
  (params (WeaponChange :type BP%20Weapon%20Base%20Object%20Reference))
  (bind _player (Variables|Default|GetPlayer))
  (bind _player_2 (Variables|Default|GetPlayer))
  (bind _player_3 (Variables|Default|GetPlayer))
  (bind _mesh (Variables|/Script/Engine.Character|GetMesh _player_3))
  (Variables|/Game/MyGameContent/Player/BP_Player.BP_Player_C|SetIsAiming _player_2 false)
  (Variables|/Game/MyGameContent/Player/BP_Player.BP_Player_C|SetIsFire _player_2 false)
  (Animation|Montage|PlayMontage _mesh (Variables|Default|GetAnimUnEquip)
    (:OnCompleted
      (CallFunction|FAttachWeapon WeaponChange)
      (Animation|Montage|PlayMontage _mesh (Variables|Default|GetAnimEquip)
        (:OnCompleted
          (Variables|/Game/MyGameContent/Player/BP_Player.BP_Player_C|SetIsEquip _player false)
          (bind _output_get (Variables|/Game/MyGameContent/Player/BP_Player.BP_Player_C|SetCurrentWeapon _player WeaponChange))
          (CallFunction|GetPose _output_get)
          (CallFunction|GetHudAmmoNow _output_get)
          (CallFunction|GetHudAmmoHave _output_get))))))

(event Custom|GetPose)

(event Custom|Throw/Aim_End
  (Variables|/Script/Engine.CharacterMovementComponent|SetMaxWalkSpeed (Variables|/Script/Engine.Character|GetCharacterMovement (Variables|Default|GetPlayer)) 6e+02))

(event Custom|Throwing)

(event Custom|Throw/Aim_Start
  (Variables|/Script/Engine.CharacterMovementComponent|SetMaxWalkSpeed (Variables|/Script/Engine.Character|GetCharacterMovement (Variables|Default|GetPlayer)) 3e+02))

(event Custom|GetHudAmmoNow)

(event Custom|GetHudAmmoHave)

(event EventBeginPlay
  (bind _asbp_player (Utilities|Casting|CastToBP_Player (Game|GetPlayerCharacter 0)))
  (Variables|Default|SetPlayer _asbp_player))

(fn ConstructionScript
  (Variables|Default|SetUpgradeRecoil 1.0))

(fn FAttachWeapon
  (params (WeaponChenge :type BP%20Weapon%20Base%20Object%20Reference))
  (Transformation|AttachComponentToComponent WeaponChenge (Variables|/Script/Engine.Character|GetMesh (Variables|Default|GetPlayer)) "skt_gun" "SnapToTarget" "KeepRelative" "KeepRelative" true)
  (Transformation|AttachComponentToComponent self (Variables|/Script/Engine.Character|GetMesh (Variables|Default|GetPlayer)) "skt_back1" "SnapToTarget" "KeepRelative" "KeepRelative" true)
  (return))