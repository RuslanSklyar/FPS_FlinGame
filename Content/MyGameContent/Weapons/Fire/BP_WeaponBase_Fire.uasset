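; Base Blueprint for player firearms, handling single and automatic fire, montage-timed reloads, timeline-driven recoil and aim zoom, and HUD ammo updates.
; The construction script copies stats, mesh, sounds and montages from the DASettings data asset.
; Each shot traces for muzzle obstruction, then from the camera with random spray, with a conditional muzzle re-trace.
; It spawns BP_Bullet at the resulting hit location, carrying damage, plus a Niagara tracer.
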(event Custom|Reload
  (if (!= (Variables|DA_Settings|GetAmmoNow) (Variables|DA_Settings|GetAmmoInClip))
    (if (> (Variables|DA_Settings|GetAmmoHave) 0)
      (if (not (Variables|Default|GetIsReload))
        (Variables|Default|SetIsReload true)
        (CallFunction|Throw/AimEnd)
        (Default|FCrossViis (Variables|Default|GetPlayer))
        (bind _reloaddelay (CallFunction|FPlayMotage false (Variables|DA_Settings|GetWeaponReloadMontage) (Variables|DA_Settings|GetPlayer%20Reload%20Montage)))
        (Utilities|FlowControl|Delay _reloaddelay)
        (CallFunction|FCalculateReload))
      (else
        (CallFunction|FPlayerReloadFalse :!label _label)))
    (else
      (goto _label))))

(event EventBeginPlay
  (|CallParentFunction))

(event Collision|EventActorBeginOverlap
  (params (OtherActor :type Actor%20Object%20Reference))
  (|CallParentFunction OtherActor))

(event EventTick
  (params (DeltaSeconds :type Float%20%28single-precision%29))
  (|CallParentFunction DeltaSeconds))

(event EventFire
  (params (Fire :type Boolean))
  (if Fire :!label _label
    (if (not (Variables|Default|GetIsFire))
      (if (> (Variables|DA_Settings|GetAmmoNow) 0)
        (Variables|Default|SetIsFire true)
        (CallFunction|WeaponRecoil)
        (CallFunction|FFireFX)
        (switch Utilities|FlowControl|Switch|SwitchonE_FireMode (Variables|DA_Settings|GetWeapon%20Fire%20Mode)
          (:NewEnumerator0
            (Utilities|MFireLogic))
          (:NewEnumerator1
            (Utilities|MFireLogic)
            (goto _label)))
        (elif (> (Variables|DA_Settings|GetAmmoHave) 0)
          (CallFunction|Reload))))))

(event EventWeaponRecoil
  (bind _lenght (Timeline|Recoil Play)
    (:Update
      (Pawn|Input|AddControllerPitchInput (Variables|Default|GetPlayer) (* (* _lenght (select (Variables|/Game/MyGameContent/Player/BP_Player.BP_Player_C|GetIsCrouch (Variables|Default|GetPlayer)) (- (Variables|DA_Settings|GetFireRecoil) 0.06) (Variables|DA_Settings|GetFireRecoil))) (Variables|Default|GetUpgradeRecoil)))
      (Pawn|Input|AddControllerYawInput (Variables|Default|GetPlayer) (* (* (* _lenght (select (Variables|/Game/MyGameContent/Player/BP_Player.BP_Player_C|GetIsCrouch (Variables|Default|GetPlayer)) (- (Variables|DA_Settings|GetFireRecoil) 0.06) (Variables|DA_Settings|GetFireRecoil))) (Variables|Default|GetUpgradeRecoil)) (select (Math|Random|RandomBool) 1.0 -1.0))))))

(event EventThrow/AimStart
  (bind _player (Variables|Default|GetPlayer))
  (|CallParentFunction)
  (Default|ScopeScale (Variables|/Game/MyGameContent/Player/BP_Player.BP_Player_C|GetWD_Cross _player))
  (Variables|/Game/MyGameContent/Player/BP_Player.BP_Player_C|SetIsAiming _player true)
  (bind _newtrack_0 (Timeline|Timeline_0 Play)
    (:Update
      (Variables|/Script/Engine.CameraComponent|SetFieldOfView (Variables|/Game/MyGameContent/Player/BP_Player.BP_Player_C|GetFollowCamera _player) _newtrack_0))))

(event EventGetPose
  (Variables|/Game/MyGameContent/Player/BP_Player.BP_Player_C|SetWeaponPose (Variables|Default|GetPlayer) (Variables|DA_Settings|GetWeapon%20Pose)))

(event EventThrow/AimEnd
  (bind _player (Variables|Default|GetPlayer))
  (|CallParentFunction)
  (Variables|/Game/MyGameContent/Player/BP_Player.BP_Player_C|SetIsAiming _player false)
  (bind _newtrack_0 (Timeline|Timeline_0 Reverse)
    (:Update
      (Variables|/Script/Engine.CameraComponent|SetFieldOfView (Variables|/Game/MyGameContent/Player/BP_Player.BP_Player_C|GetFollowCamera _player) _newtrack_0))))

(event EventGetHudAmmoHave
  (Default|WeaponAmmoHave (Variables|/Game/MyGameContent/Player/HUD/Widgets/WD_MainHud.WD_MainHud_C|GetWD_WeaponHud (Variables|/Game/MyGameContent/Player/BP_Player.BP_Player_C|GetWD_MainHud (Variables|Default|GetPlayer))) (Variables|DA_Settings|GetAmmoHave) (Variables|DA_Settings|GetWeapon%20Pose)))

(event EventGetHudAmmoNow
  (Default|WeaponAmmoNow (Variables|/Game/MyGameContent/Player/HUD/Widgets/WD_MainHud.WD_MainHud_C|GetWD_WeaponHud (Variables|/Game/MyGameContent/Player/BP_Player.BP_Player_C|GetWD_MainHud (Variables|Default|GetPlayer))) (Variables|DA_Settings|GetAmmoNow) (Variables|DA_Settings|GetWeapon%20Pose)))

(fn ConstructionScript
  (bind _da_settings (Variables|DA_Settings|GetDA_Settings))
  (bind _da_settings_2 (Variables|DA_Settings|GetDA_Settings))
  (|CallParentFunction)
  (if (Utilities|IsValid (Variables|DA_Settings|GetDA_Settings))
    (Variables|DA_Settings|SetCanScope (Variables|/Game/MyGameContent/Weapons/Fire/PDA_WeaponFire.PDA_WeaponFire_C|GetCanScope _da_settings))
    (Variables|DA_Settings|SetMuzzleName (Variables|/Game/MyGameContent/Weapons/Fire/PDA_WeaponFire.PDA_WeaponFire_C|GetMuzzleName _da_settings))
    (Variables|DA_Settings|SetAmmoMax (Variables|/Game/MyGameContent/Weapons/Fire/PDA_WeaponFire.PDA_WeaponFire_C|GetAmmoMax _da_settings))
    (Variables|DA_Settings|SetAmmoNow (Variables|/Game/MyGameContent/Weapons/Fire/PDA_WeaponFire.PDA_WeaponFire_C|GetAmmoNow _da_settings))
    (Variables|DA_Settings|SetAmmoInClip (Variables|/Game/MyGameContent/Weapons/Fire/PDA_WeaponFire.PDA_WeaponFire_C|GetAmmoInClip _da_settings))
    (Variables|DA_Settings|SetAmmoHave (Variables|/Game/MyGameContent/Weapons/Fire/PDA_WeaponFire.PDA_WeaponFire_C|GetAmmoHave _da_settings))
    (Variables|DA_Settings|SetFireRate (Variables|/Game/MyGameContent/Weapons/Fire/PDA_WeaponFire.PDA_WeaponFire_C|GetFireRate _da_settings))
    (Variables|DA_Settings|SetFireRecoil (Variables|/Game/MyGameContent/Weapons/Fire/PDA_WeaponFire.PDA_WeaponFire_C|GetFireRecoil _da_settings))
    (Variables|DA_Settings|SetFireSpray (Variables|/Game/MyGameContent/Weapons/Fire/PDA_WeaponFire.PDA_WeaponFire_C|GetFireSpray _da_settings))
    (Variables|DA_Settings|SetFireDamage (Variables|/Game/MyGameContent/Weapons/Fire/PDA_WeaponFire.PDA_WeaponFire_C|GetFireDamage _da_settings))
    (Class|SkinnedMeshComponent|SetSkeletalMesh (Variables|Default|GetWeaponSkelet) (Variables|/Game/MyGameContent/Weapons/Fire/PDA_WeaponFire.PDA_WeaponFire_C|GetSkelet _da_settings) true)
    (Variables|DA_Settings|SetSound%20Fire (Variables|/Game/MyGameContent/Weapons/Fire/PDA_WeaponFire.PDA_WeaponFire_C|GetSoundFire _da_settings_2))
    (Variables|DA_Settings|SetSoundReload (Variables|/Game/MyGameContent/Weapons/Fire/PDA_WeaponFire.PDA_WeaponFire_C|GetSoundReload _da_settings_2))
    (Variables|DA_Settings|SetSound%20No%20Ammo (Variables|/Game/MyGameContent/Weapons/Fire/PDA_WeaponFire.PDA_WeaponFire_C|GetSoundNoAmmo _da_settings_2))
    (Variables|DA_Settings|SetWeaponFireMotage (Variables|/Game/MyGameContent/Weapons/Fire/PDA_WeaponFire.PDA_WeaponFire_C|GetWeaponFireMotage _da_settings_2))
    (Variables|DA_Settings|SetWeaponReloadMontage (Variables|/Game/MyGameContent/Weapons/Fire/PDA_WeaponFire.PDA_WeaponFire_C|GetWeaponReloadMontage _da_settings_2))
    (Variables|DA_Settings|SetPlayer%20Fire%20Montage (Variables|/Game/MyGameContent/Weapons/Fire/PDA_WeaponFire.PDA_WeaponFire_C|GetPlayerFireMontage _da_settings_2))
    (Variables|DA_Settings|SetPlayer%20Reload%20Montage (Variables|/Game/MyGameContent/Weapons/Fire/PDA_WeaponFire.PDA_WeaponFire_C|GetPlayerReloadMontage _da_settings_2))
    (Variables|DA_Settings|SetWeapon%20Pose (Variables|/Game/MyGameContent/Weapons/Fire/PDA_WeaponFire.PDA_WeaponFire_C|GetWeaponPose _da_settings_2))
    (Variables|DA_Settings|SetWeapon%20Fire%20Mode (Variables|/Game/MyGameContent/Weapons/Fire/PDA_WeaponFire.PDA_WeaponFire_C|GetWeaponFireMode _da_settings_2))
    (Transformation|SetRelativeLocation (Variables|Default|GetMuzzlePoint) (Transformation|GetSocketLocation (Variables|Default|GetWeaponSkelet) (Variables|DA_Settings|GetMuzzleName)) true true)))

(fn FSpawnFire
  (bind _result (Math|Integer|DecrementInt (Variables|DA_Settings|GetAmmoNow))
    (:%20%20
      (Variables|DA_Settings|SetAmmoNow _result)
      (CallFunction|FPlayMotage false (Variables|DA_Settings|GetWeaponFireMotage) (Variables|DA_Settings|GetPlayer%20Fire%20Montage))
      (CallFunction|FLineTrace)
      (CallFunction|GetHudAmmoNow)
      (Default|ScopeFire (Variables|/Game/MyGameContent/Player/BP_Player.BP_Player_C|GetWD_Cross (Variables|Default|GetPlayer))))))

(fn FLineTrace
  (bind _player (Variables|Default|GetPlayer))
  (bind _weaponskelet (Variables|Default|GetWeaponSkelet))
  (bind _muzzlename (Variables|DA_Settings|GetMuzzleName))
  (bind _muzzlename_2 (Variables|DA_Settings|GetMuzzleName))
  (bind _weaponskelet_2 (Variables|Default|GetWeaponSkelet))
  (bind _returnvalue (Transformation|GetSocketLocation _weaponskelet _muzzlename))
  (bind _returnvalue_2 (Transformation|GetSocketLocation _weaponskelet_2 _muzzlename_2))
  (bind _followcamera (Variables|/Game/MyGameContent/Player/BP_Player.BP_Player_C|GetFollowCamera _player))
  (bind _returnvalue_3 (Transformation|GetWorldLocation _followcamera))
  (bind (_outhit _returnvalue_4) (Collision|LineTraceByChannel _returnvalue_2 (+ _returnvalue_2 (* (Math|Vector|GetForwardVector (Transformation|GetSocketRotation _weaponskelet_2 _muzzlename_2)) 5e+01)) "TraceTypeQuery1" false 0 "None"))
  (if _returnvalue_4
    (Variables|Default|SetOut%20Hit _outhit)
    (CallFunction|FSpawnBullet)
    (else
      (bind _outhit_2 (Collision|LineTraceByChannel _returnvalue_3 (Math|Random|RandomPointinBoundingBox (+ _returnvalue_3 (* (Math|Vector|GetForwardVector _followcamera) 1e+05)) (* "1.000000,1.000000,1.000000" (Variables|DA_Settings|GetFireSpray))) "TraceTypeQuery1" false (Utilities|Array|MakeArray self (Game|GetInstigator)) "None"))
      (if (Utilities|DoesObjectImplementInterface (.HitActor (Collision|BreakHitResult _outhit_2)) "/Game/MyGameContent/BPI/BPI_GetCharacters.BPI_GetCharacters_C")
        (Variables|Default|SetOut%20Hit _outhit_2)
        (CallFunction|FSpawnBullet)
        (elif (Utilities|MGetTraceVector (Math|Vector|SelectVector (.Location (Collision|BreakHitResult _outhit_2)) (.TraceEnd (Collision|BreakHitResult _outhit_2)) (.bBlockingHit (Collision|BreakHitResult _outhit_2))))
          (bind _outhit_3 (Collision|LineTraceByChannel _returnvalue (Math|Random|RandomPointinBoundingBox (+ _returnvalue (* (Math|Vector|GetForwardVector (Transformation|GetSocketRotation (Variables|Default|GetWeaponSkelet) (Variables|DA_Settings|GetMuzzleName))) 1e+05)) (* "1.000000,1.000000,1.000000" (Variables|DA_Settings|GetFireSpray))) "TraceTypeQuery1" false 0 "None"))
          (Variables|Default|SetOut%20Hit _outhit_3)
          (CallFunction|FSpawnBullet)
          (else
            (Variables|Default|SetOut%20Hit _outhit_2)
            (CallFunction|FSpawnBullet)))))))

(fn FTraceFX
  (params (InValue :type Vector))
  (bind _returnvalue (Niagara|SpawnSystematLocation "/Game/MyGameContent/Weapons/Fire/VFX/NS_FireTrace.NS_FireTrace" (Transformation|GetSocketLocation (Variables|Default|GetWeaponSkelet) (Variables|DA_Settings|GetMuzzleName))))
  (Class|NiagaraComponent|SetNiagaraVariableVec3 _returnvalue "TraceTarget" InValue))

(fn FPlayMotage
  (params (WeaponAnim? :type Boolean) (MontageWeapon :type Anim%20Montage%20Object%20Reference) (MontagePlayer :type Anim%20Montage%20Object%20Reference))
  (if WeaponAnim?
    (Animation|Montage|MontagePlay (Components|SkeletalMesh|GetAnimInstance (Variables|Default|GetWeaponSkelet)) MontageWeapon 1.0 "MontageLength" 0.0 true)
    (bind _returnvalue (Animation|Montage|MontagePlay (Components|SkeletalMesh|GetAnimInstance (Variables|/Script/Engine.Character|GetMesh (Variables|Default|GetPlayer))) MontagePlayer 1.0 "MontageLength" 0.0 true))
    (return _returnvalue)
    (else
      (bind _returnvalue_2 (Animation|Montage|MontagePlay (Components|SkeletalMesh|GetAnimInstance (Variables|/Script/Engine.Character|GetMesh (Variables|Default|GetPlayer))) MontagePlayer 1.0 "MontageLength" 0.0 true))
      (return _returnvalue_2))))

(fn FCalculateReload
  (bind _output_get (LocalVariables|SetNeedAmmo (- (Variables|DA_Settings|GetAmmoInClip) (Variables|DA_Settings|GetAmmoNow))))
  (if (> _output_get (Variables|DA_Settings|GetAmmoHave))
    (Variables|DA_Settings|SetAmmoNow (+ (Variables|DA_Settings|GetAmmoHave) (Variables|DA_Settings|GetAmmoNow)))
    (Variables|DA_Settings|SetAmmoHave 0)
    (else
      (Variables|DA_Settings|SetAmmoNow (+ (Variables|DA_Settings|GetAmmoNow) (LocalVariables|GetNeedAmmo)))
      (Variables|DA_Settings|SetAmmoHave (- (Variables|DA_Settings|GetAmmoHave) (LocalVariables|GetNeedAmmo)))))
  (Variables|Default|SetIsReload false)
  (Variables|/Game/MyGameContent/Player/BP_Player.BP_Player_C|SetIsReload (Variables|Default|GetPlayer) false)
  (CallFunction|GetHudAmmoHave)
  (CallFunction|GetHudAmmoNow))

(fn FPlayerReloadFalse
  (Variables|/Game/MyGameContent/Player/BP_Player.BP_Player_C|SetIsReload (Variables|Default|GetPlayer) false))

(fn FFireFX
  (bind _weaponskelet (Variables|Default|GetWeaponSkelet))
  (bind _muzzlename (Variables|DA_Settings|GetMuzzleName))
  (bind _returnvalue (Transformation|GetSocketLocation _weaponskelet _muzzlename))
  (Audio|PlaySoundatLocation (Variables|DA_Settings|GetSound%20Fire) _returnvalue "0, 0, 0" 1.0 1.0 0.0 0 0 0)
  (Effects|SpawnEmitteratLocation "/Game/MyGameContent/Weapons/Fire/VFX/P_MuzzleFlash.P_MuzzleFlash" _returnvalue (Transformation|GetSocketRotation _weaponskelet _muzzlename)))

(fn FSpawnBullet
  (bind _out_hit (Variables|Default|GetOut%20Hit))
  (bind (_bblockinghit _binitialoverlap _time _distance _location _impactpoint _normal _impactnormal _physmat _hitactor _hitcomponent _hitbonename _hititem _elementindex _faceindex _tracestart _traceend) (Collision|BreakHitResult _out_hit))
  (bind _returnvalue (Math|Vector|SelectVector _location _traceend _bblockinghit))
  (Game|SpawnActorfromClass "/Game/MyGameContent/Weapons/Fire/Bullet/Blueprints/BP_Bullet.BP_Bullet_C" (Math|Transform|MakeTransform _location (Math|Rotator|FindLookatRotation _location _returnvalue)) "Undefined" 0 (Variables|DA_Settings|GetFireDamage) (Game|GetInstigator))
  (CallFunction|FTraceFX _returnvalue))