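; Base Blueprint for thrown weapons such as grenades, handling aiming with a trajectory preview and the throw itself.
; Aim start plays the toss montage, whose notify starts a looping SpawnThrow that predicts the projectile path from control rotation and rebuilds spline meshes along the player's GrenadeSpline.
; Fire ends aiming, detaches the actor and launches ProjectileMovement at the predicted velocity, while ending aim without firing just clears the preview and montage.
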(event Custom|ThrowGrenade
  (Components|Activation|SetActive (Variables|Default|GetProjectileMovement) true false)
  (Transformation|DetachFromActor "KeepWorld" "KeepRelative" "KeepRelative")
  (Variables|/Script/Engine.MovementComponent|SetVelocity (Variables|Default|GetProjectileMovement) (Variables|Default|GetProjectileVelocity)))

(event Custom|SpawnThrow
  (bind _returnvalue (Math|Float|MakeLiteralFloat 0.03))
  (bind _player (Variables|Default|GetPlayer))
  (CallFunction|ClearSplineMesh)
  (if (Variables|/Game/MyGameContent/Player/BP_Player.BP_Player_C|GetIsThrow _player)
    (bind _output_get (Variables|Default|SetProjectileVelocity (* (+ (Math|Vector|GetForwardVector (Pawn|GetControlRotation _player :!class /Script/Engine.Pawn)) "0,0.000000,1.000000") 7e+02)))
    (bind _outpathpositions (Class|GameplayStatics|BlueprintPredictProjectilePathbyTraceChannel (Transformation|GetWorldLocation (Variables|/Game/MyGameContent/Player/BP_Player.BP_Player_C|GetGrenadePossThrow (Variables|Default|GetPlayer))) _output_get true 0.0 "ECC_Camera" false (Utilities|Array|MakeArray (Variables|Default|GetPlayer)) "None" 3e+01))
    (for (_array_element _array_index) _outpathpositions
      (Spline|AddSplinePointatIndex (Variables|/Game/MyGameContent/Player/BP_Player.BP_Player_C|GetGrenadeSpline (Variables|Default|GetPlayer)) _array_element _array_index "Local" true))
    (for _index (range 0 (- (Spline|GetNumberOfSplinePoints (Variables|/Game/MyGameContent/Player/BP_Player.BP_Player_C|GetGrenadeSpline (Variables|Default|GetPlayer))) 2))
      (bind _returnvalue_2 (AddComponent|AddSplineMeshComponent true))
      (SplineMesh|SetStartScale _returnvalue_2 (Math|Vector2D|MakeVector2D _returnvalue _returnvalue) true :!class /Script/Engine.SplineMeshComponent)
      (SplineMesh|SetEndScale _returnvalue_2 (Math|Vector2D|MakeVector2D _returnvalue _returnvalue) true :!class /Script/Engine.SplineMeshComponent)
      (Utilities|Array|Add (Variables|Default|GetSplineMeshComponent) _returnvalue_2)
      (SplineMesh|SetStartandEnd _returnvalue_2 (.ReturnValue (Utilities|PosThrow _index)) (.ReturnValue2 (Utilities|PosThrow _index)) (.ReturnValue3 (Utilities|PosThrow _index)) (.ReturnValue4 (Utilities|PosThrow _index)) true :!class /Script/Engine.SplineMeshComponent))
    (Utilities|FlowControl|Delay 0.03)
    (CallFunction|SpawnThrow)))

(event EventFire
  (params (Fire :type Boolean))
  (if Fire
    (Variables|Default|SetIsFire true)
    (CallFunction|Throw/AimEnd)
    (Development|PrintString "fire")))

(event EventThrow/AimStart
  (|CallParentFunction)
  (if (not (Variables|/Game/MyGameContent/Player/BP_Player.BP_Player_C|GetIsThrowing (Variables|Default|GetPlayer)))
    (Animation|Montage|PlayMontage (Variables|/Script/Engine.Character|GetMesh (Variables|Default|GetPlayer)) "/Game/MyGameContent/Player/Animations/Montage/Toss_Grenade_Montage.Toss_Grenade_Montage" 1.0 0.0 "Throwing"
      (:OnNotifyBegin
        (Variables|/Game/MyGameContent/Player/BP_Player.BP_Player_C|SetIsThrow (Variables|Default|GetPlayer) true)
        (CallFunction|SpawnThrow)))))

(event EventThrow/AimEnd
  (|CallParentFunction)
  (if (Variables|Default|GetIsFire)
    (Variables|/Game/MyGameContent/Player/BP_Player.BP_Player_C|SetIsThrowing (Variables|Default|GetPlayer) true)
    (Animation|Montage|PlayMontage (Variables|/Script/Engine.Character|GetMesh (Variables|Default|GetPlayer)) "/Game/MyGameContent/Player/Animations/Montage/Toss_Grenade_Montage.Toss_Grenade_Montage" 1.5 0.0 "End"
      (:then
        (Variables|/Game/MyGameContent/Player/BP_Player.BP_Player_C|SetIsThrow (Variables|Default|GetPlayer) false)
        (CallFunction|ThrowGrenade)
        (Animation|StopAnimMontage (Variables|Default|GetPlayer) 0 :!label _label)
        (Variables|/Game/MyGameContent/Player/BP_Player.BP_Player_C|SetIsThrowing (Variables|Default|GetPlayer) false)
        (Variables|/Game/MyGameContent/Player/BP_Player.BP_Player_C|SetIsThrow (Variables|Default|GetPlayer) false)
        (CallFunction|ClearSplineMesh)
        (Variables|Default|SetIsFire false))
      (:OnCompleted
        (Variables|/Game/MyGameContent/Player/BP_Player.BP_Player_C|SetIsThrowing (Variables|Default|GetPlayer) true)))
    (else
      (goto _label))))

(fn ConstructionScript
  (|CallParentFunction))

(fn ClearSplineMesh
  (bind _splinemeshcomponent (Variables|Default|GetSplineMeshComponent))
  (Spline|ClearSplinePoints (Variables|/Game/MyGameContent/Player/BP_Player.BP_Player_C|GetGrenadeSpline (Variables|Default|GetPlayer)) true)
  (for _array_element _splinemeshcomponent
    (Components|DestroyComponent _array_element))
  (Utilities|Array|Clear _splinemeshcomponent))