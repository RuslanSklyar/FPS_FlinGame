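; BP_Grenade is a throwable grenade weapon that deals area damage when it explodes.
; ThrowGrenade runs the parent throw, then after a short delay enables physics on the skeleton and sphere.
; Hit calls Boom and destroys the actor; Boom asks the GS_GrenadeAOEDamage game state to spawn a line-of-sight-checked area effect.
; Its hit delegate, TakeDamage, applies fixed damage through each hit actor's GetHealthMessage result.
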(event Custom|Boom
  (bind _asgs_grenade_aoedamage (Utilities|Casting|CastToGS_GrenadeAOEDamage (Game|GetGameState)))
  (Default|SpawnAOE _asgs_grenade_aoedamage (Transformation|GetActorLocation) 6e+02 true self (delegate Custom|TakeDamage)))

(event Custom|TakeDamage
  (params (HitActor :type Actor%20Object%20Reference))
  (bind _bpc_health (Class|BPIGetCharacters|GetHealth(Message) HitActor))
  (Default|FTakeDamage _bpc_health "None" 1.5e+02))

(event EventBeginPlay
  (|CallParentFunction))

(event Collision|EventActorBeginOverlap
  (params (OtherActor :type Actor%20Object%20Reference))
  (|CallParentFunction OtherActor) ; This node is disabled and will not be called.\nDrag off pins to build functionality.
)

(event EventTick
  (params (DeltaSeconds :type Float%20%28single-precision%29))
  (|CallParentFunction DeltaSeconds))

(event Collision|EventHit
  (params (MyComp :type Primitive%20Component%20Object%20Reference) (Other :type Actor%20Object%20Reference) (OtherComp :type Primitive%20Component%20Object%20Reference) (bSelfMoved :type Boolean) (HitLocation :type Vector :default "0, 0, 0") (HitNormal :type Vector :default "0, 0, 0") (NormalImpulse :type Vector :default "0, 0, 0") (Hit :type Hit%20Result%20Structure%20%28by%20ref%29))
  (CallFunction|Boom)
  (Actor|DestroyActor))

(event EventThrowGrenade
  (|CallParentFunction)
  (Utilities|FlowControl|Delay 0.2)
  (Physics|SetSimulatePhysics (Variables|Default|GetWeaponSkelet) true))

(fn ConstructionScript
  (|CallParentFunction))

(fn GetCharacter
  (return 0))