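; Character component that tracks health, applies hit and fall damage, and handles death.
; Hits, with tenfold damage on the head, change a buffer value that Health follows at constant speed for the HP bar, snapping on headshots or depletion.
; Tick converts vertical speed into a fall-damage fraction, applied on landing.
; At zero health, the capsule loses collision and the mesh ragdolls, with its bodies put to sleep three seconds later.
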(event Custom|CustomEvent
  (params (BoneName :type Name) (Damage :type Float%20%28single-precision%29) (Instigator :type Actor%20Object%20Reference)))

(event Custom|OnDeath
  (bind _player (Variables|Default|GetPlayer))
  (bind _player_2 (Variables|Default|GetPlayer))
  (bind _mesh (Variables|/Script/Engine.Character|GetMesh _player_2))
  (bind _mesh_2 (Variables|/Script/Engine.Character|GetMesh _player))
  (Collision|SetCollisionEnabled (Variables|/Script/Engine.Character|GetCapsuleComponent (Variables|Default|GetPlayer)) "NoCollision")
  (Class|SkeletalMeshComponent|SetAllBodiesSimulatePhysics _mesh true)
  (Collision|SetCollisionProfileName _mesh "Ragdoll" false :!class /Script/Engine.PrimitiveComponent)
  (Variables|Default|SetIsAlive false)
  (Utilities|FlowControl|Delay 3.0)
  (for _array_element (Transformation|GetAllSocketNames _mesh_2)
    (Class|PrimitiveComponent|PutRigidBodytoSleep _mesh_2 _array_element)))

(event Custom|AddHealth
  (params (AddHealth :type Float%20%28single-precision%29))
  ;[1 1 1] Event Damage
  ;;[1 1 1] Изменение ХП Playera
  (Variables|Default|SetHealthBuffer (+ AddHealth (Variables|Default|GetHealthBuffer))))

(event Custom|CalculetHealth
  (params (DeltaTime :type Float%20%28single-precision%29))
  ;[1 1 1] Event Damage
  ;;[1 1 1] Посчёт разници HP для HP Bar
  (if (or (Variables|Default|GetHead) (<= (Variables|Default|GetHealthBuffer) 0.0))
    (Variables|Default|SetHealth (Variables|Default|GetHealthBuffer))
    (else
      (Variables|Default|SetHealth (Math|Interpolation|FInterptoConstant (Variables|Default|GetHealth) (Variables|Default|GetHealthBuffer) DeltaTime 75.0)))))

(event Custom|CheckFallDamage
  ;[1 1 1] Event Damage
  ;;[1 1 1] Система урона от падения
  (Variables|Default|SetFallDamage (Math|Float|Clamp(Float) (Math|Float|NormalizetoRange (Math|Float|Absolute(Float) (.Z (Math|Vector|BreakVector (Transformation|GetVelocity (Variables|Default|GetPlayer))))) 8e+02 1.2e+03))))

(event Custom|F_TakeDamage
  (params (BoneName :type Name) (Damage :type Float%20%28single-precision%29))
  (bind _returnvalue (* Damage -1.0))
  ;[1 1 1] Получение урона персонажа
  (Variables|Default|SetHead (Utilities|Name|Equal(Name) BoneName "head"))
  (CallFunction|AddHealth (Math|Float|SelectFloat (* _returnvalue 1e+01) _returnvalue (Variables|Default|GetHead))))

(event Custom|OnLanded
  ;[1 1 1] Event Damage
  ;;[1 1 1] Просчет урона от падения
  (if (> (Variables|Default|GetFallDamage) 0.0)
    (if (== (Variables|Default|GetFallDamage) 1.0)
      (CallFunction|AddHealth (* (Variables|Default|GetHealth) -1.0))
      (else
        (CallFunction|AddHealth (* (* (Variables|Default|GetHealthMax) (Variables|Default|GetFallDamage)) -1.0))))))

(event EventBeginPlay)

(event EventTick
  (params (DeltaSeconds :type Float%20%28single-precision%29))
  (if (Variables|Default|GetIsAlive)
    (if (> (Variables|Default|GetHealth) 0.0)
      (CallFunction|CheckFallDamage)
      (CallFunction|CalculetHealth DeltaSeconds)
      (else
        (CallFunction|OnDeath)))))

(fn FInit
  (params (CharRef :type Character%20Object%20Reference) (Health :type Float%20%28single-precision%29))
  (Variables|Default|SetPlayer CharRef)
  (bind _output_get (Variables|Default|SetHealth Health))
  (Variables|Default|SetHealthBuffer _output_get))