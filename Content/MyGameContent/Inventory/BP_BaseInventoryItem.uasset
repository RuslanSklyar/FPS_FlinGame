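; Base pickup actor for inventory items, with an inspection view for items flagged as needing it.
; The construction script loads item properties from a DT_InventoryItem row.
; A highlight volume caches the player via GetPlayerMessage; an interact volume toggles input and shows a HUD prompt.
; Take blends the camera to the item, locks movement and look, and lights a spotlight; TakeOut reverses this, and no inventory transfer is implemented.
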(event OnComponentBeginOverlap(CollisionHighlight)
  (params (OverlappedComponent :type Primitive%20Component%20Object%20Reference) (OtherActor :type Actor%20Object%20Reference) (OtherComp :type Primitive%20Component%20Object%20Reference) (OtherBodyIndex :type Integer) (bFromSweep :type Boolean) (SweepResult :type Hit%20Result%20Structure%20%28by%20ref%29))
  (bind _player (Class|BPIGetCharacters|GetPlayer(Message) OtherActor))
  (bind _output_get (Variables|Default|SetPlayer _player))
  (if (Utilities|IsValid _output_get)
    _))

(event OnComponentEndOverlap(CollisionHighlight)
  (params (OverlappedComponent :type Primitive%20Component%20Object%20Reference) (OtherActor :type Actor%20Object%20Reference) (OtherComp :type Primitive%20Component%20Object%20Reference) (OtherBodyIndex :type Integer))
  (if (== OtherActor (Variables|Default|GetPlayer))
    (Variables|Default|SetPlayer 0)))

(event OnComponentBeginOverlap(CollisionInteract)
  (params (OverlappedComponent :type Primitive%20Component%20Object%20Reference) (OtherActor :type Actor%20Object%20Reference) (OtherComp :type Primitive%20Component%20Object%20Reference) (OtherBodyIndex :type Integer) (bFromSweep :type Boolean) (SweepResult :type Hit%20Result%20Structure%20%28by%20ref%29))
  (if (== OtherActor (Variables|Default|GetPlayer))
    (Input|EnableInput (Game|GetPlayerController 0))
    (Class|BPIHud|ShowTip(Message) (HUD|GetHUD (Game|GetPlayerController 0)) "Press <Input>E</> to Interact" 5.0)))

(event OnComponentEndOverlap(CollisionInteract)
  (params (OverlappedComponent :type Primitive%20Component%20Object%20Reference) (OtherActor :type Actor%20Object%20Reference) (OtherComp :type Primitive%20Component%20Object%20Reference) (OtherBodyIndex :type Integer))
  (if (== OtherActor (Variables|Default|GetPlayer))
    (Input|DisableInput (Game|GetPlayerController 0))))

(event Custom|Take
  (bind _returnvalue (Game|GetPlayerController 0))
  (if (Variables|InventoryDataInfo|GetNeed%20Inspecting%20to%20Take)
    (Game|Player|SetViewTargetwithBlend (Game|GetPlayerController 0) self 1.0 "VTBlend_Cubic" 0.0 true)
    (Input|SetIgnoreLookInput _returnvalue true)
    (Input|SetIgnoreMoveInput _returnvalue true)
    (Rendering|SetVisibility (Variables|Default|GetSpotLight) true false)))

(event Custom|TakeOut
  (Game|Player|SetViewTargetwithBlend (Game|GetPlayerController 0) (Variables|Default|GetPlayer) 1.0 "VTBlend_Cubic" 0.0 true)
  (Class|Controller|ResetIgnoreInputFlags (Game|GetPlayerController 0))
  (Rendering|SetVisibility (Variables|Default|GetSpotLight) false false))

(event Input|ActionEvents|InputActionInteract
  (params (Key :type Key%20Structure))
  (:Pressed
    (CallFunction|Take)))

(fn ConstructionScript
  (bind _returnvalue (Utilities|GetDataTableRow "/Game/MyGameContent/Inventory/DT_InventoryItem.DT_InventoryItem" (Variables|InventoryDataInfo|GetRow%20Name))
    (:then
      (Variables|InventoryDataInfo|SetName (.Name (Utilities|Struct|BreakStruct_InventoryItem _returnvalue)))
      (Variables|InventoryDataInfo|SetDescription (.Description (Utilities|Struct|BreakStruct_InventoryItem _returnvalue)))
      (Variables|InventoryDataInfo|SetNeed%20Inspecting%20to%20Take (.NeedInspectingToTake (Utilities|Struct|BreakStruct_InventoryItem _returnvalue)))
      (Variables|InventoryDataInfo|SetCan%20be%20Stack (.CanBeStack (Utilities|Struct|BreakStruct_InventoryItem _returnvalue)))
      (Variables|InventoryDataInfo|SetCategory (.Category (Utilities|Struct|BreakStruct_InventoryItem _returnvalue))))))

(fn GetBPC
  (return 0))

(fn GetCharacter
  (return 0))