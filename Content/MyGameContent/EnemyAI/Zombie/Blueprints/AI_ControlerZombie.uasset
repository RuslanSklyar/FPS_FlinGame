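; AI controller for the zombie enemy that starts the BT_Zombie behavior tree on possession.
; GetPlayer queries the perception component for actors sensed by sight and uses a GetPlayerForAIMessage call to identify the player.
; The loop returns on its first iteration, so only the first perceived actor is checked, yielding that actor or nothing.
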(event EventPossess
  (params (PossessedPawn :type Pawn%20Object%20Reference))
  (AI|RunBehaviorTree "/Game/MyGameContent/EnemyAI/Zombie/AI/BT_Zombie.BT_Zombie"))

(fn ConstructionScript
  (|CallParentFunction))

(fn GetPlayer
  (bind _aiperception (Variables|Default|GetAIPerception))
  (bind _outactors (Class|AIPerceptionComponent|GetPerceivedActors _aiperception "/Script/AIModule.AISense_Sight"))
  (if (!= (Utilities|Array|Length _outactors) 0)
    (for _array_element _outactors
      (bind _isplayer (Class|BPIAITargetPlayer|GetPlayerforAI(Message) _array_element))
      (if _isplayer
        (return _array_element)
        (else
          (return 0))))
    (else
      (return 0))))