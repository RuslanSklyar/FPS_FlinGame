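; BP_EnemyBase is a base enemy character Blueprint that hosts health, blood and inventory components.
; On BeginPlay it initialises the health component with itself and a starting health value, and it forwards landing events to that component when valid.
; Getter functions expose the three components and the character itself, while GetPlayer returns no value and Tick and construction are empty.
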(event EventBeginPlay
  (Default|FInit (Variables|Default|GetBPC_Health) self 1e+02))

(event EventOnLanded
  (params (Hit :type Hit%20Result%20Structure%20%28by%20ref%29))
  (bind _bpc_health (Variables|Default|GetBPC_Health))
  (Utilities|IsValid _bpc_health
    (:Is%20Valid
      (Default|OnLanded _bpc_health))))

(event EventTick
  (params (DeltaSeconds :type Float%20%28single-precision%29)))

(fn ConstructionScript)

(fn GetBlood
  (return (Variables|Default|GetBPC_Blood)))

(fn GetCharacters
  (return self))

(fn GetHealth
  (return (Variables|Default|GetBPC_Health)))

(fn GetInventory
  (return (Variables|Default|GetBPC_Inventory)))

(fn GetPlayer
  (return 0))